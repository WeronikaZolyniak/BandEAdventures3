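; Moving platform actor that shuttles back and forth between its placed location and a target location at a set speed.
; BeginPlay converts TargetLocation, an offset from the actor's position, into world space without applying actor rotation.
; Tick moves it along the normalized direction without sweep, swapping start and target once the distance travelled reaches the journey length, with no clamping at endpoints.
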(event EventBeginPlay
  (Variables|Default|SetCurrentStartLocation (Transformation|GetActorLocation))
  (Variables|Default|SetCurrentTargetLocation (Math|Transform|TransformLocation (Math|Conversions|ToTransform(Vector) (Transformation|GetActorLocation)) (Variables|Default|GetTargetLocation))))

(event EventTick
  (params (DeltaSeconds :type Float%20%28single-precision%29))
  (Variables|Default|SetLocation (Transformation|GetActorLocation))
  (Variables|Default|SetJourneyLength (Math|Vector|VectorLength (- (Variables|Default|GetCurrentTargetLocation) (Variables|Default|GetCurrentStartLocation))))
  (Variables|Default|SetJourneyTravelled (Math|Vector|VectorLength (- (Variables|Default|GetLocation) (Variables|Default|GetCurrentStartLocation))))
  (if (>= (Variables|Default|GetJourneyTravelled) (Variables|Default|GetJourneyLength))
    (Variables|Default|SetSwap (Variables|Default|GetCurrentStartLocation))
    (Variables|Default|SetCurrentStartLocation (Variables|Default|GetCurrentTargetLocation))
    (Variables|Default|SetCurrentTargetLocation (Variables|Default|GetSwap))
    (Variables|Default|SetDirection (Math|Vector|Normalize (- (Variables|Default|GetCurrentTargetLocation) (Variables|Default|GetCurrentStartLocation))))
    (Transformation|SetActorLocation (+ (Transformation|GetActorLocation) (* (Variables|Default|GetDirection) (* DeltaSeconds (Variables|Default|GetSpeed)))) false false)
    (else
      (Variables|Default|SetDirection (Math|Vector|Normalize (- (Variables|Default|GetCurrentTargetLocation) (Variables|Default|GetCurrentStartLocation))))
      (Transformation|SetActorLocation (+ (Transformation|GetActorLocation) (* (Variables|Default|GetDirection) (* DeltaSeconds (Variables|Default|GetSpeed)))) false false))))

(fn ConstructionScript)