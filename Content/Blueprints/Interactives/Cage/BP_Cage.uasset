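; BP_Cage is a kickable 2D cage holding an instrument, which either of two players can break.
; Once the game mode reports players spawned, it binds to both players' kick events.
; A kick from a player overlapping its collision swaps the cage to a destroyed flipbook and hides the instrument.
; Index selects the instrument flipbook on BeginPlay, though every case uses the same test asset; Interact is empty.
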(event Custom|Kick
  (params (player%20ref :type BP%20Player%20Base%20Object%20Reference))
  ;[1 1 1] binding destroying function
  (if (Collision|IsOverlappingActor (Variables|Default|GetCollision) player%20ref :!class /Script/Engine.PrimitiveComponent)
    (CallFunction|CageDestroyed)))

(event Custom|Bindtokick
  ;[1 1 1] binding destroying function
  (bind _asbp_player_base (Utilities|Casting|CastToBP_PlayerBase (Game|GetPlayerCharacter 0)))
  (EventDispatchers|BindEventtoKick _asbp_player_base (delegate Custom|Kick))
  (bind _asbp_player_base_2 (Utilities|Casting|CastToBP_PlayerBase (Game|GetPlayerCharacter 1)))
  (EventDispatchers|BindEventtoKick _asbp_player_base_2 (delegate Custom|Kick)))

(event EventBeginPlay
  (bind _fb_test (Variables|Default|GetFB_Test))
  (bind _instrument (Variables|Default|GetInstrument))
  (Utilities|FlowControl|Sequence
    (:then_0
      ;[1 1 1] binding destroying function
      (bind _asbp_game_mode_base (Utilities|Casting|CastToBP_GameModeBase (Game|GetGameMode)))
      (EventDispatchers|BindEventtoPlayersSpawned _asbp_game_mode_base (delegate Custom|Bindtokick)))
    (:then_1
      (switch int (Variables|Default|GetIndex)
        (:0
          (Sprite|SetFlipbook _instrument _fb_test))
        (:1
          (Sprite|SetFlipbook _instrument _fb_test))
        (:2
          (Sprite|SetFlipbook _instrument _fb_test))
        (:3
          (Sprite|SetFlipbook _instrument _fb_test))
        (:4
          (Sprite|SetFlipbook _instrument _fb_test))
        (:5
          (Sprite|SetFlipbook _instrument _fb_test))
        (:6
          (Sprite|SetFlipbook _instrument _fb_test))
        (:7
          (Sprite|SetFlipbook _instrument _fb_test))
        (:8
          (Sprite|SetFlipbook _instrument _fb_test))
        (:9
          (Sprite|SetFlipbook _instrument _fb_test))))))

(event Collision|EventActorBeginOverlap
  (params (OtherActor :type Actor%20Object%20Reference)))

(event EventTick
  (params (DeltaSeconds :type Float%20%28single-precision%29)))

(fn ConstructionScript)

(fn Interact
  (params (PlayerRef :type BP%20Player%20Base%20Object%20Reference)))

(fn CageDestroyed
  (Sprite|SetFlipbook (Variables|Default|GetCage) "/Game/Assets/Flipbooks/Interactives/FB_CageDestroyed.FB_CageDestroyed")
  (Rendering|SetVisibility (Variables|Default|GetInstrument) false false))