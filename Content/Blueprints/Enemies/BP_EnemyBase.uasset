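; Base enemy Blueprint that reacts to the player touching its capsule by turning and throwing a placeholder punch.
; On capsule overlap, an IsPlayer interface message identifies the player, and their relative Y position picks one of two opposite rotations.
; After a short delay it only prints "Punch", with no damage applied.
; UpdateFlipbooks, the construction script and the other events are empty stubs.
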(event OnComponentBeginOverlap(CapsuleComponent)
  (params (OverlappedComponent :type Primitive%20Component%20Object%20Reference) (OtherActor :type Actor%20Object%20Reference) (OtherComp :type Primitive%20Component%20Object%20Reference) (OtherBodyIndex :type Integer) (bFromSweep :type Boolean) (SweepResult :type Hit%20Result%20Structure%20%28by%20ref%29))
  (bind _yes_no (Class|BPIPlayer|IsPlayer(Message) OtherActor))
  (if _yes_no
    (if (>= (- (.y (Transformation|GetActorLocation OtherActor)) (.y (Transformation|GetActorLocation))) 0.0)
      (Transformation|SetActorRotation "0,90.000000, 0")
      (Utilities|FlowControl|Delay 0.75)
      (Development|PrintString "Punch")
      (else
        (Transformation|SetActorRotation "0,-90.000000, 0")
        (Utilities|FlowControl|Delay 0.75)
        (Development|PrintString "Punch")))))

(event EventBeginPlay)

(event Collision|EventActorBeginOverlap
  (params (OtherActor :type Actor%20Object%20Reference)))

(event EventTick
  (params (DeltaSeconds :type Float%20%28single-precision%29)))

(fn ConstructionScript)

(fn UpdateFlipbooks)