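; BP_Brett is a 2D side-scrolling character with flipbook animation and wall sliding.
; Each tick it pins X to the movement plane, refreshes grounded state, updates the sprite and flips control yaw to match horizontal velocity.
; Hanging and punching flipbooks override those chosen by movement state: idle, walk, jump or slide.
; While airborne, wall detection with low or downward vertical velocity starts sliding; otherwise sliding stops.
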(event EventBeginPlay
  (Variables|Default|SetMovementState "NewEnumerator3"))

(event EventTick
  (params (DeltaSeconds :type Float%20%28single-precision%29))
  (bind _returnvalue (Transformation|GetActorLocation))
  (Transformation|SetActorLocation (Math|Vector|MakeVector 0.0 (.y _returnvalue) (.z _returnvalue)) false false)
  (CallFunction|SetIsGrounded)
  (Utilities|FlowControl|Sequence
    (:then_0
      (CallFunction|UpdateFlipbooks))
    (:then_1
      (CallFunction|UpdatePlayerRotation))
    (:then_2
      (if (not (Variables|Default|GetIsGrounded))
        (bind (_returnvalue_2 _wallnormal) (CallFunction|WallDetector 5.0))
        (if (and _returnvalue_2 (< (.z (Transformation|GetVelocity)) 2e+01))
          (Variables|Default|SetWallNormal _wallnormal)
          (CallFunction|Slide)
          (else
            (CallFunction|StopSliding)))))))

(fn ConstructionScript
  (|CallParentFunction))

(fn UpdateFlipbooks
  (if (Variables|Default|GetIsHanging)
    (Sprite|SetFlipbook (Variables|Default|GetSprite) (Variables|Default|GetFB_Hang))
    (elif (Variables|Default|GetIsPunching)
      (Sprite|SetFlipbook (Variables|Default|GetSprite) (Variables|Default|GetFB_Punch))
      (else
        (Variables|Default|SetMovementState (select (and (Variables|Default|GetIsSliding) (not (Variables|Default|GetIsGrounded))) "NewEnumerator4" (select (Variables|Default|GetIsGrounded) (select (!= 0.0 (Variables|Default|GetAxisValueMoveRight)) "NewEnumerator1" "NewEnumerator0") "NewEnumerator2")))
        (Sprite|SetFlipbook (Variables|Default|GetSprite) (Utilities|Select :Index (Variables|Default|GetMovementState) :NewEnumerator3 0 :NewEnumerator0 (Variables|Default|GetFB_Idle) :NewEnumerator1 (Variables|Default|GetFB_Walk) :NewEnumerator2 (Variables|Default|GetFB_Jump) :NewEnumerator4 (Variables|Default|GetFB_Slide)))))))

(fn UpdatePlayerRotation
  (Math|Float|CompareFloat (.y (Transformation|GetVelocity)) 0.0
    (:>
      (Pawn|SetControlRotation (Game|GetPlayerController (Variables|Default|GetIndex)) (Math|Rotator|MakeRotator 0.0 0.0 0.0)))
    (:<
      (Pawn|SetControlRotation (Game|GetPlayerController (Variables|Default|GetIndex)) (Math|Rotator|MakeRotator 0.0 0.0 1.8e+02)))))