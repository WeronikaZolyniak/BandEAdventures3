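; Game Instance that loads, applies and saves audio volume options, reapplying them on Init.
; Load Options fetches or creates an SV_Options save object, whose values ReloadAudioSettings sends through the SaveAudioSettings message.
; SaveAudioSettings maps volume indices to levels, sets sound mix overrides and writes the options to the save slot.
; All three overrides target the Master sound class, including music and SFX; SpawnPlayer only returns false.
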(event EventSaveAudioSettings
  (params (master%20vol :type Integer) (music%20vol :type Integer) (sfx%20vol :type Integer))
  (bind _sv_options (Variables|Default|GetSV%20Options))
  (Audio|SetSoundMixClassOverride "/Game/Audio/SoundClasses/MasterMix.MasterMix" "/Game/Audio/SoundClasses/Master.Master" (Utilities|Select :Index master%20vol :Option%200 0.1 :Option%201 0.2 :Option%202 0.3 :Option%203 0.4 :Option%204 0.5 :Option%205 0.6 :Option%206 0.7 :Option%207 0.8 :Option%208 0.9 :Option%209 1.0) 1.0 1.0 true)
  (Audio|SetSoundMixClassOverride "/Game/Audio/SoundClasses/MasterMix.MasterMix" "/Game/Audio/SoundClasses/Master.Master" (Utilities|Select :Index music%20vol :Option%200 0.1 :Option%201 0.2 :Option%202 0.3 :Option%203 0.4 :Option%204 0.5 :Option%205 0.6 :Option%206 0.7 :Option%207 0.8 :Option%208 0.9 :Option%209 1.0) 1.0 1.0 true)
  (Audio|SetSoundMixClassOverride "/Game/Audio/SoundClasses/MasterMix.MasterMix" "/Game/Audio/SoundClasses/Master.Master" (Utilities|Select :Index sfx%20vol :Option%200 0.1 :Option%201 0.2 :Option%202 0.3 :Option%203 0.4 :Option%204 0.5 :Option%205 0.6 :Option%206 0.7 :Option%207 0.8 :Option%208 0.9 :Option%209 1.0) 1.0 1.0 true)
  (Utilities|LoadOptions
    (:OutputPin
      (Variables|/Game/Blueprints/SaveFiles/SV_Options.SV_Options_C|Setmaster%20vol _sv_options master%20vol)
      (Variables|/Game/Blueprints/SaveFiles/SV_Options.SV_Options_C|Setmusic%20vol _sv_options music%20vol)
      (Variables|/Game/Blueprints/SaveFiles/SV_Options.SV_Options_C|Setsfx%20vol _sv_options sfx%20vol)
      (SaveGame|SaveGametoSlot (Variables|Default|GetSV%20Options) (Variables|Default|Getoption%20save%20slot)))))

(event EventInit
  (CallFunction|ReloadAudioSettings))

(fn ReloadAudioSettings
  (bind _sv_options (Utilities|LoadOptions)
    (:OutputPin
      (Class|BPIGameMode|SaveAudioSettings(Message) self (Variables|/Game/Blueprints/SaveFiles/SV_Options.SV_Options_C|Getmaster%20vol _sv_options) (Variables|/Game/Blueprints/SaveFiles/SV_Options.SV_Options_C|Getmusic%20vol _sv_options) (Variables|/Game/Blueprints/SaveFiles/SV_Options.SV_Options_C|Getsfx%20vol _sv_options)))))

(fn SpawnPlayer
  (params (CurrentPlayerIndex :type Integer) (InputReceiver :type BP%20Input%20Reciever%20Object%20Reference))
  (return false))